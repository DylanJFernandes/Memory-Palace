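; Castle double door Blueprint that swings open when a Character begins overlapping it and closes when one stops overlapping.
; The overlap events set an Open flag, with no count of how many characters remain inside.
; Tick steps Angle toward the open or closed target at a fixed speed, snapping when within one step, and yaws the left and right pivots in opposite directions.
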(event EventBeginPlay)

(event Collision|EventActorBeginOverlap
  (params (OtherActor :type Actor%20Object%20Reference))
  (Utilities|Casting|CastToCharacter OtherActor)
  (Variables|Default|SetbOpen true))

(event EventTick
  (params (DeltaSeconds :type Float%20%28single-precision%29))
  (bind _returnvalue (Math|Float|MakeLiteralFloat 105.0))
  (bind _returnvalue_2 (Math|Float|MakeLiteralFloat 0.0))
  (bind _returnvalue_3 (Math|Float|MakeLiteralFloat 1.4e+02))
  (bind _bopen (Variables|Default|GetbOpen))
  (bind _returnvalue_4 (* DeltaSeconds _returnvalue_3))
  (bind _returnvalue_5 (select _bopen _returnvalue _returnvalue_2))
  (Variables|Default|SetAngle (select (> (- _returnvalue_5 (Variables|Default|GetAngle)) _returnvalue_4) (+ (Variables|Default|GetAngle) _returnvalue_4) (select (< (- _returnvalue_5 (Variables|Default|GetAngle)) (- (Math|Float|MakeLiteralFloat 0.0) _returnvalue_4)) (- (Variables|Default|GetAngle) _returnvalue_4) _returnvalue_5)))
  (Transformation|SetRelativeRotation (Variables|Default|GetPivotL) (Math|Rotator|MakeRotator 0.0 0.0 (- (Math|Float|MakeLiteralFloat 0.0) (select (> (- _returnvalue_5 (Variables|Default|GetAngle)) _returnvalue_4) (+ (Variables|Default|GetAngle) _returnvalue_4) (select (< (- _returnvalue_5 (Variables|Default|GetAngle)) (- (Math|Float|MakeLiteralFloat 0.0) _returnvalue_4)) (- (Variables|Default|GetAngle) _returnvalue_4) _returnvalue_5)))) false false)
  (Transformation|SetRelativeRotation (Variables|Default|GetPivotR) (Math|Rotator|MakeRotator 0.0 0.0 (select (> (- _returnvalue_5 (Variables|Default|GetAngle)) _returnvalue_4) (+ (Variables|Default|GetAngle) _returnvalue_4) (select (< (- _returnvalue_5 (Variables|Default|GetAngle)) (- (Math|Float|MakeLiteralFloat 0.0) _returnvalue_4)) (- (Variables|Default|GetAngle) _returnvalue_4) _returnvalue_5))) false false))

(event Collision|EventActorEndOverlap
  (params (OtherActor :type Actor%20Object%20Reference))
  (Utilities|Casting|CastToCharacter OtherActor)
  (Variables|Default|SetbOpen false))

(fn ConstructionScript)